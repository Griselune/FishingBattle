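; Fishing ground actor that drives a Niagara effect aligned to the height of the surface at its location.
; On BeginPlay it line traces on the Visibility channel from above the Niagara component down to its origin to find the surface Z.
; That height is passed to the effect's WaterZ parameter, then the effect is activated.
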(event EventBeginPlay
  (bind _serface (CallFunction|GetSerfaceHeight))
  (Niagara|SetNiagaraVariable(Float) (Variables|Default|GetNiagara) "WaterZ" _serface)
  (Components|Activation|SetActive (Variables|Default|GetNiagara) true false))

(event Collision|EventActorBeginOverlap
  (params (OtherActor :type Actor%20Object%20Reference)))

(event EventTick
  (params (DeltaSeconds :type Float%20%28single-precision%29)))

(fn ConstructionScript)

(fn GetSerfaceHeight
  (bind _niagara (Variables|Default|GetNiagara))
  (bind _returnvalue (Transformation|GetWorldLocation _niagara))
  (bind (_outhit _returnvalue_2) (Collision|LineTraceByChannel (+ (* (Math|Vector|GetUpVector _niagara) 1e+03) _returnvalue) _returnvalue "TraceTypeQuery1" false 0 "None"))
  (if _returnvalue_2
    (return (.Z (Math|Vector|BreakVector (.Location (Collision|BreakHitResult _outhit)))))))