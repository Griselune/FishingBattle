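; BP_SpotTarget is an actor that hops between BP_ResultPlayer actors like a roulette, then settles on the winner.
; Start gathers the players and snaps to a random one, then a looping timeline lerps it to another randomly picked player.
; Once Tick's timer reaches TimeLimit, the target index switches to the player whose UUID matches Winner.
; When the timeline next finishes, it calls Finished instead of looping.
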(event Custom|Move
  (Variables|Default|SetCurrentLocation (Transformation|GetActorLocation) :!label _label)
  (bind _speed (Timeline|MoveProcess PlayFromStart)
    (:Update
      (Transformation|SetActorLocation (Math|Vector|Lerp(Vector) (Variables|Default|GetCurrentLocation) (Transformation|GetActorLocation (Utilities|Array|Get(acopy) (Variables|Default|GetPlayers) (Variables|Default|GetPlayer%20Index))) _speed) false false))
    (:Finished
      (if (not (Variables|Default|GetNeedStop))
        (bind _playerindex (CallFunction|GetRandomTarget))
        (Variables|Default|SetPlayer%20Index _playerindex)
        (goto _label)
        (else
          (Default|CallFinished))))))

(event Custom|Start
  (bind _outactors (Actor|GetAllActorsOfClass "/Game/WuBranch/Actor/BP_ResultPlayer.BP_ResultPlayer_C"))
  (Variables|Default|SetPlayers _outactors)
  (CallFunction|InitLocation)
  (bind _playerindex (CallFunction|GetRandomTarget))
  (Variables|Default|SetPlayer%20Index _playerindex)
  (Variables|Default|SetCanStart true)
  (CallFunction|Move))

(event EventBeginPlay)

(event Collision|EventActorBeginOverlap
  (params (OtherActor :type Actor%20Object%20Reference)))

(event EventTick
  (params (DeltaSeconds :type Float%20%28single-precision%29))
  (if (Variables|Default|GetCanStart)
    (bind _output_get (Variables|Default|SetMoveTime (+ DeltaSeconds (Variables|Default|GetMoveTime))))
    (if (>= _output_get (Variables|Default|GetTimeLimit))
      (Variables|Default|SetNeedStop true)
      (bind _index (CallFunction|GetWinnerIndex (Variables|Default|GetWinner)))
      (Variables|Default|SetPlayer%20Index _index))))

(fn ConstructionScript)

(fn GetRandomTarget
  (bind _players (Variables|Default|GetPlayers))
  (bind _returnvalue (Utilities|Array|Length _players))
  ;[0.15 0.15 0.15 0.5] データがない場合エラーログを出す
  (if (!= _returnvalue 0)
    ;[0.15 0.15 0.15 0.5] 一つだけの場合、直接0の方をあげる
    (if (> _returnvalue 1)
      ;[0.15 0.15 0.15 0.5] 二つ以上の場合、ランダムであげる
      (LocalVariables|SetNew%20Target (Math|Random|RandomInteger _returnvalue) :!label _label)
      (if (== (LocalVariables|GetNew%20Target) (Variables|Default|GetPlayer%20Index))
        (goto _label)
        (else
          (return (LocalVariables|GetNew%20Target))))
      (else
        (return 0)))
    (else
      (Development|PrintString "Error! No Player Data" false true "(R=1.000000,G=0.029910,B=0.000000,A=1.000000)" 1.0))))

(fn GetWinner)

(fn InitLocation
  (bind _playerindex (CallFunction|GetRandomTarget))
  (Variables|Default|SetPlayer%20Index _playerindex)
  (Transformation|SetActorLocation (Transformation|GetActorLocation (Utilities|Array|Get(acopy) (Variables|Default|GetPlayers) (Variables|Default|GetPlayer%20Index))) false false))

(fn GetWinnerIndex
  (params (TargetID :type Integer))
  (bind (_array_element _array_index) (Utilities|Array|ForEachLoopwithBreak (Variables|Default|GetPlayers) :!label _label)
    (:LoopBody
      (if (== (Variables|/Game/WuBranch/Actor/BP_ResultPlayer.BP_ResultPlayer_C|GetUUID _array_element) TargetID)
        (LocalVariables|SetTarget _array_index)
        (goto _label Break)))
    (:Completed
      (return (LocalVariables|GetTarget)))))

(fn SetWinner
  (params (Winner :type Integer))
  (Variables|Default|SetWinner Winner))