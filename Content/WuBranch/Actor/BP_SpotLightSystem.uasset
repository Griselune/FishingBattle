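; BP_SpotLightSystem runs the winner reveal show, coordinating spotlights, audio, fireworks and the result UI.
; On BeginPlay it gathers lights, targets and fireworks, then chains pre-reveal, cheers and claps sounds through audio-finished callbacks.
; Each Tick it aims each light at the same-index target, provided both counts match.
; When all targets report finished, it activates every firework and calls ShowWinner on WBP_Result widgets inside that loop.
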(event Custom|OnFinish
  (bind _result (Math|Integer|IncrementInt (Variables|Default|GetFinishedTargetNum))
    (:%20%20
      (if (== _result (Utilities|Array|Length (Variables|Default|GetTarget)))
        (for _array_element (Variables|Default|GetFireworks)
          (Default|MultiActivate _array_element)
          (bind _foundwidgets (Widget|GetAllWidgetsOfClass "/Game/WuBranch/UI/WBP_Result.WBP_Result_C" true))
          (if (Utilities|Array|IsNotEmpty _foundwidgets)
            (for _array_element_2 _foundwidgets
              (Default|ShowWinner _array_element_2))))))))

(event Custom|OnRevealFinish
  (bind _returnvalue (Audio|CreateSound2D "/Game/WuBranch/Sound/Cue/A_CheersAndClaps_Cue.A_CheersAndClaps_Cue" 1.0 1.0 0.0 0))
  (EventDispatchers|BindEventtoOnAudioFinished _returnvalue (delegate Custom|OnCheersFinish))
  (Audio|Components|Audio|Play _returnvalue 0.0))

(event Custom|OnCheersFinish
  (bind _returnvalue (Audio|CreateSound2D "/Game/WuBranch/Sound/Cue/A_Claps_Cue.A_Claps_Cue" 1.0 1.0 0.0 0))
  (Audio|Components|Audio|Play _returnvalue 0.0))

(event EventBeginPlay
  (bind _outactors (Actor|GetAllActorsOfClass "/Game/WuBranch/Actor/BP_Light.BP_Light_C"))
  (Variables|Default|SetLights _outactors)
  (bind _outactors_2 (Actor|GetAllActorsOfClass "/Game/WuBranch/Actor/BP_SpotTarget.BP_SpotTarget_C"))
  (bind _output_get (Variables|Default|SetTarget _outactors_2))
  (for _array_element _output_get
    (EventDispatchers|BindEventtoFinished _array_element (delegate Custom|OnFinish)))
  (bind _outactors_3 (Actor|GetAllActorsOfClass "/Game/WuBranch/Actor/BP_Firework.BP_Firework_C"))
  (Variables|Default|SetFireworks _outactors_3)
  (bind _returnvalue (Audio|CreateSound2D "/Game/WuBranch/Sound/Cue/A_Pre-reveal_Cue.A_Pre-reveal_Cue" 1.0 1.0 0.0 0))
  (EventDispatchers|BindEventtoOnAudioFinished _returnvalue (delegate Custom|OnRevealFinish))
  (Audio|Components|Audio|Play _returnvalue 0.0))

(event Collision|EventActorBeginOverlap
  (params (OtherActor :type Actor%20Object%20Reference)))

(event EventTick
  (params (DeltaSeconds :type Float%20%28single-precision%29))
  (if (== (Utilities|Array|Length (Variables|Default|GetLights)) (Utilities|Array|Length (Variables|Default|GetTarget)))
    (CallFunction|FacetoTarget)))

(fn ConstructionScript)

(fn FacetoTarget
  (for (_array_element _array_index) (Variables|Default|GetLights)
    (bind _spotlight (Default|GetLight _array_element))
    (Transformation|SetWorldRotation _spotlight (Math|Rotator|FindLookatRotation (Transformation|GetWorldLocation _spotlight) (Transformation|GetActorLocation (Utilities|Array|Get(acopy) (Variables|Default|GetTarget) _array_index))) false false)))