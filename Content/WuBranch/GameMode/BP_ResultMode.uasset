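; BP_ResultMode is the result-screen game mode, with helpers to pick a match winner and spawn result players.
; FindPotentials keeps the GameInstance records with the fewest deaths, and GetWinner breaks ties by highest total damage.
; SpawnPlayer places a BP_ResultPlayer yawed toward the camera, and DecideLocation supplies random points in a flat box.
; BeginPlay calls none of these, and CreateUI's WBP_Result widget logic is disconnected.
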(event EventBeginPlay)

(event EventTick
  (params (DeltaSeconds :type Float%20%28single-precision%29)))

(fn ConstructionScript)

(fn SpawnPlayer
  (params (Location :type Vector))
  (bind _returnvalue (Game|SpawnActorfromClass "/Game/WuBranch/Actor/BP_ResultPlayer.BP_ResultPlayer_C" (Math|Transform|MakeTransform Location (Math|Rotator|MakeRotator 0.0 0.0 (.yaw (Math|Rotator|FindLookatRotation Location (Variables|Default|GetCameraLocation)))) "1.000000,1.000000,1.000000") "Undefined" "MultiplyWithRoot" 0 0))
  (return _returnvalue))

(fn DecideLocation
  (return (Math|Random|RandomPointinBoundingBox "0.000000,0.000000,118.000000" "200.000000,200.000000,0.000000")))

(fn GetWinner
  (params (Potentials :type Array%20of%20Player%20Record%20Structures))
  (bind _output (Utilities|Array|Get(acopy) Potentials))
  ;[0.15 0.15 0.15 0.5] １人の場合
  (if (> (Utilities|Array|Length Potentials) 1)
    ;[0.15 0.15 0.15 0.5] 一番与えたダメージが多い人が勝つ
    (LocalVariables|SetMaxDamage (.totaldamage _output))
    (LocalVariables|SetWinnerID (.id _output))
    (LocalVariables|SetWinnerName (.name _output))
    (for _array_element Potentials
      (if (> (.totaldamage _array_element) (LocalVariables|GetMaxDamage))
        (LocalVariables|SetMaxDamage (.totaldamage _array_element))
        (LocalVariables|SetWinnerID (.id _array_element))
        (LocalVariables|SetWinnerName (.name _array_element))))
    (return (LocalVariables|GetWinnerID) (LocalVariables|GetWinnerName))
    (else
      (return (.id _output) (.name _output)))))

(fn FindPotentials
  (bind _gameinstance (Variables|Default|GetGameInstance))
  (bind _returnvalue (Class|LANGameInstance|GetRecords _gameinstance))
  (LocalVariables|SetMinDeathCount (.deathcount (Utilities|Array|Get(acopy) _returnvalue)))
  (for _array_element _returnvalue
    (if (== (.DeathCount (Utilities|Struct|BreakPlayerRecord _array_element)) (LocalVariables|GetMinDeathCount))
      (Utilities|Array|Add (LocalVariables|GetLocalPotentials) _array_element :!label _label)
      (elif (< (.DeathCount (Utilities|Struct|BreakPlayerRecord _array_element)) (LocalVariables|GetMinDeathCount))
        (Utilities|Array|Clear (LocalVariables|GetLocalPotentials))
        (LocalVariables|SetMinDeathCount (.DeathCount (Utilities|Struct|BreakPlayerRecord _array_element)))
        (goto _label))))
  (return (LocalVariables|GetLocalPotentials)))

(fn CreateUI
  (params (Winner%20Name :type String)))